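; Checkpoint manager for a lap-based race that tracks progress and reports laps to MyHUD.
; A single trigger box hops to the next of eight checkpoint transforms whenever an overlap ends, with a delayed DoOnce blocking repeat triggers.
; After the eighth count it increments the lap and either returns to the first checkpoint, checking the lap record and resetting lap time, or sets the HUD's RaceOver flag to false past the maximum.
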(event `self.ReceiveBeginPlay`
  (bind _asmy_hud (cast `/Game/Blueprints/MyHud` (`PlayerController.GetHUD` (`GameplayStatics.GetPlayerController` 0))))
  (set `/Game/Blueprints/MyHud.HUD_Lap` (`self.LAP`) _asmy_hud)
  (set `/Game/Blueprints/MyHud.HUD_MaxLaps` (`self.MAXLAPS`) _asmy_hud))

(event `self.CP_TriggerBox_0.OnComponentEndOverlap`
  (params (OtherActor :type "Actor Object Reference") (OtherComp :type "PrimitiveComponent Object Reference") (OtherBodyIndex :type Integer))
  (if (== (`self.CP_COUNT`) 8)
    (`KismetSystemLibrary.Delay` 0.2)
    (set `self.CP_COUNT` 1)
    (set `self.LAP` (+ 1 (`self.LAP`)))
    (if (<= (`self.LAP`) (`self.MAXLAPS`))
      ;[1 1 1] Moves Triggerbox to Starting Checkpoint
      (`SceneComponent.K2_SetWorldTransform` (`self.CP_TriggerBox_0`) (`SceneComponent.K2_GetComponentToWorld` (`self.CP_1_0`)) false)
      (bind _asmy_hud (cast `/Game/Blueprints/MyHud` (`PlayerController.GetHUD` (`GameplayStatics.GetPlayerController` 0))))
      (set `/Game/Blueprints/MyHud.HUD_Lap` (`self.LAP`) _asmy_hud)
      (`/Game/Blueprints/MyHud.LapRecordCheck` _asmy_hud)
      (`KismetSystemLibrary.Delay` 0.2)
      (`/Game/Blueprints/MyHud.ResetLapTime` _asmy_hud)
      (else
        (bind _asmy_hud_2 (cast `/Game/Blueprints/MyHud` (`PlayerController.GetHUD` (`GameplayStatics.GetPlayerController` 0))))
        (set `/Game/Blueprints/MyHud.RaceOver` false _asmy_hud_2)))
    (else
      (`/Engine/EditorBlueprintResources/StandardMacros.DoOnce` false :!label _label
        (:`Completed`
          (`SceneComponent.K2_SetWorldTransform` (`self.CP_TriggerBox_0`) (`SceneComponent.K2_GetComponentToWorld` (`KismetArrayLibrary.Array_Get` (`|MakeArray` (`self.CP_1_0`) (`self.CP_2_0`) (`self.CP_3_0`) (`self.CP_4_0`) (`self.CP_5_0`) (`self.CP_6_0`) (`self.CP_7_0`) (`self.CP_8_0`)) (`self.CP_COUNT`))) false)
          (set `self.CP_COUNT` (+ 1 (`self.CP_COUNT`)))
          (`KismetSystemLibrary.Delay` 1.0)
          (goto _label :!via `Reset`))))))

(fn `UserConstructionScript`)