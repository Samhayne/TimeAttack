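; Actor that persists best lap and race times for a racing game and shows them on the HUD.
; On BeginPlay it loads the BP_SaveGame slot and copies the times into MyHUD, or creates and saves one with default times if none exists.
; Pressing R before the race starts reuses that default-creation branch to reset saved and displayed times, limited to once by a DoOnce.
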(event `self.ReceiveBeginPlay`
  (bind _bp_savegame (`self.BP_Savegame`))
  (`self.EnableInput` (`GameplayStatics.GetPlayerController` 0))
  (bind _returnvalue (`GameplayStatics.DoesSaveGameExist` "SaveGameSlot"))
  (if _returnvalue
    (bind _returnvalue_2 (`GameplayStatics.LoadGameFromSlot` "SaveGameSlot"))
    (set `self.BP_Savegame` _returnvalue_2)
    ;[1 1 1] Loads the Best Times and Laps
    (bind _asbp_save_game (cast `/Game/Blueprints/BP_SaveGame` _bp_savegame))
    (bind _asmy_hud (cast `/Game/Blueprints/MyHud` (`PlayerController.GetHUD` (`GameplayStatics.GetPlayerController` 0))))
    (set `/Game/Blueprints/MyHud.H Best Lap Min` (`/Game/Blueprints/BP_SaveGame.S BestLapMin` _asbp_save_game) _asmy_hud)
    (set `/Game/Blueprints/MyHud.H Best Lap Sec` (`/Game/Blueprints/BP_SaveGame.S BestLapSec` _asbp_save_game) _asmy_hud)
    (set `/Game/Blueprints/MyHud.H Best Time Min` (`/Game/Blueprints/BP_SaveGame.S BestTimeMin` _asbp_save_game) _asmy_hud)
    (set `/Game/Blueprints/MyHud.H Best Time Sec` (`/Game/Blueprints/BP_SaveGame.S BestTimeSec` _asbp_save_game) _asmy_hud)
    (else
      (bind _returnvalue_3 (`GameplayStatics.CreateSaveGameObject` "/Game/Blueprints/BP_SaveGame.BP_SaveGame_C" :!label _label))
      (set `self.BP_Savegame` _returnvalue_3)
      ;[1 1 1] Reserzs the Best Times to Default
      (bind _asbp_save_game_2 (cast `/Game/Blueprints/BP_SaveGame` _bp_savegame))
      (set `/Game/Blueprints/BP_SaveGame.S BestLapMin` (`self.D BestLapMin`) _asbp_save_game_2)
      (set `/Game/Blueprints/BP_SaveGame.S BestLapSec` (`self.D BestLapSec`) _asbp_save_game_2)
      (set `/Game/Blueprints/BP_SaveGame.S BestTimeMin` (`self.D BestTimeMin`) _asbp_save_game_2)
      (set `/Game/Blueprints/BP_SaveGame.S BestTimeSec` (`self.D BestTimeSec`) _asbp_save_game_2)
      (`GameplayStatics.SaveGameToSlot` _bp_savegame "SaveGameSlot")
      ;[1 1 1] Updates the HUD with the default values
      (bind _asmy_hud_2 (cast `/Game/Blueprints/MyHud` (`PlayerController.GetHUD` (`GameplayStatics.GetPlayerController` 0))))
      (set `/Game/Blueprints/MyHud.H Best Lap Min` (`self.D BestLapMin`) _asmy_hud_2)
      (set `/Game/Blueprints/MyHud.H Best Lap Sec` (`self.D BestLapSec`) _asmy_hud_2)
      (set `/Game/Blueprints/MyHud.H Best Time Min` (`self.D BestTimeMin`) _asmy_hud_2)
      (set `/Game/Blueprints/MyHud.H Best Time Sec` (`self.D BestTimeSec`) _asmy_hud_2))))

(event `Key|R`
  ;[1 1 1] If the race hasn't started allow the player to reset times
  (:`Pressed`
    (bind _asmy_hud (cast `/Game/Blueprints/MyHud` (`PlayerController.GetHUD` (`GameplayStatics.GetPlayerController` 0))))
    (if (not (`/Game/Blueprints/MyHud.RaceStart` _asmy_hud))
      (`/Engine/EditorBlueprintResources/StandardMacros.DoOnce` false
        (:`Completed`
          (goto _label))))))

(fn `UserConstructionScript`)